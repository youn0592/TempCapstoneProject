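; Interactive button Blueprint for a multi-button interaction that hides a target actor when both its owner and target active states are true.
; On Interact, it queries the target interactive and both active states, disabling its own collision if either is active.
; The target actor's hidden state follows the AND of the two states, while its collision is disabled on every interaction regardless.
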(event EventInteract
  (Class|MultiButtonInteraction|GetTargetInteractive)
  (bind _returnvalue (Class|MultiButtonInteraction|GetTargetActive))
  (if _returnvalue
    (Collision|SetActorEnableCollision false))
  (bind _returnvalue_2 (Class|MultiButtonInteraction|GetTargetActor))
  (bind _returnvalue_3 (Class|MultiButtonInteraction|GetOwnerActive))
  (if _returnvalue_3
    (Collision|SetActorEnableCollision false))
  (Rendering|SetActorHiddenInGame _returnvalue_2 (and _returnvalue_3 _returnvalue))
  (Collision|SetActorEnableCollision _returnvalue_2 false))

(fn ConstructionScript)